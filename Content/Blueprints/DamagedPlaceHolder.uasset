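; A damageable placeholder sphere target that changes glow as it loses health and disappears at zero.
; BeginPlay puts a dynamic instance of MI_Target on the sphere; AnyDamage lowers clamped Health, then hides the sphere and disables its collision at zero.
; Emissive lerps by health ratio from DefaultColor at zero to DamagedColor at full health.
; The node reading DefaultColor from the material is unconnected, so it never runs.
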(event `self.ReceiveBeginPlay`
  (bind _returnvalue (`KismetMaterialLibrary.CreateDynamicMaterialInstance` "/Game/Materials/MI_Target.MI_Target"))
  (bind _output_get (set `self.Material` _returnvalue))
  (`PrimitiveComponent.SetMaterial` (`self.SphereTarget`) 0 _output_get))

(event `self.ReceiveAnyDamage`
  (params (Damage :type "Float (single-precision)") (DamageType :type "DamageType Object Reference") (InstigatedBy :type "Controller Object Reference") (DamageCauser :type "Actor Object Reference"))
  (`self.TakeDamageFromSource` Damage))

(fn `HealthUpdateColor`
  (`MaterialInstanceDynamic.SetVectorParameterValue` (`self.Material`) "Emissive" (`KismetMathLibrary.LinearColorLerp` (`self.DefaultColor`) (`self.DamagedColor`) (`KismetMathLibrary.FClamp` (/ (`self.health`) (`self.MaxHealth`))))))

(fn `TakeDamageFromSource`
  (params (B :type "Float (double-precision)"))
  (bind _output_get (set `self.health` (`KismetMathLibrary.FClamp` (- (`self.health`) B) 0.0 (`self.MaxHealth`))))
  (`self.HealthUpdateColor`)
  (if (== _output_get 0.0)
    (`SceneComponent.SetVisibility` (`self.SphereTarget`) false false)
    (`PrimitiveComponent.SetCollisionEnabled` (`self.SphereTarget`) "NoCollision")))

(fn `UserConstructionScript`)