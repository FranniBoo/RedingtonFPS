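; First-person player character with movement, look, jump and a rifle, which it spawns on BeginPlay and attaches to a gun location component.
; The Shoot axis passes a camera-forward trace segment to the equipped gun, using its max bullet distance, and gates repeat shots with a delay from its rate of fire.
; Pressing key 1 triggers a one-time oversized explosion effect with explosion and "Wow" sound effects.
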(event `Key|One`
  (params (Key :type "Key Structure"))
  (:`Pressed`
    (`/Engine/EditorBlueprintResources/StandardMacros.DoOnce` false
      (:`Completed`
        (`GameplayStatics.SpawnEmitterAtLocation` "/Game/Particles/FXBoomBoom.FXBoomBoom" (0.0 0.0 0.0) (struct) (10.0 10.0 10.0) false)
        (`GameplayStatics.PlaySound2D` "/Game/StarterContent/Audio/Explosion01.Explosion01" 1.0 1.0 0.0 null null)
        (`GameplayStatics.PlaySound2D` "/Game/Fantastic_Village_Pack/WOW_-_Eddy_Wally__Sound_Effect_HD_.WOW_-_Eddy_Wally__Sound_Effect_HD_" 1.0 1.0 0.0 null null)))))

(event `self.ReceiveBeginPlay`
  (bind _returnvalue (`|SpawnActorFromClass` "/Game/Blueprints/BPRifle.BPRifle_C" (`KismetMathLibrary.MakeTransform` (0.0 0.0 0.0) (struct) (1.25 1.25 1.25)) "Undefined" "OverrideRootScale" null null))
  (bind _output_get (set `self.EquippedGun` _returnvalue))
  (`self.K2_AttachToComponent` _output_get (`self.GunLocation`) "None" "KeepRelative" "KeepRelative" "KeepRelative" true))

(event `InputAxis|LookUpDown`
  (params (AxisValue :type "Float (single-precision)"))
  (`self.AddControllerPitchInput` AxisValue))

(event `InputAxis|MoveForwardBack`
  (params (AxisValue :type "Float (single-precision)"))
  (`self.AddMovementInput` (`self.GetActorForwardVector`) AxisValue))

(event `InputAxis|LookLeftRight`
  (params (AxisValue :type "Float (single-precision)"))
  (`self.AddControllerYawInput` AxisValue))

(event `InputAxis|MoveRightLeft`
  (params (AxisValue :type "Float (single-precision)"))
  (`self.AddMovementInput` (`self.GetActorRightVector`) AxisValue))

(event `InputAction|Jump`
  (params (Key :type "Key Structure"))
  (:`Pressed`
    (`self.Jump`)))

(event `InputAxis|Shoot`
  (params (AxisValue :type "Float (single-precision)"))
  (bind _fpscam (`self.FPSCam`))
  (bind _returnvalue (`SceneComponent.K2_GetComponentLocation` _fpscam))
  (if (and (`self.CanPlayerShoot`) (== AxisValue 1.0))
    (`/Game/Blueprints/BP_Gun_Template.Shoot` (`self.EquippedGun`) _returnvalue (+ _returnvalue (* (`SceneComponent.GetForwardVector` _fpscam) (`/Game/Blueprints/BP_Gun_Template.MaxBulletDistance` (`self.EquippedGun`)))))
    (set `self.CanPlayerShoot` false)
    (`KismetSystemLibrary.Delay` (`/Game/Blueprints/BP_Gun_Template.RateOfFire` (`self.EquippedGun`)))
    (set `self.CanPlayerShoot` true)))

(fn `UserConstructionScript`)